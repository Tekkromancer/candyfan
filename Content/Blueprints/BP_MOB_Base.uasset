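; BP_MOB_Base is a mob actor built around a physics-driven sphere, configured from a data struct and moved by velocity events.
; Initialize stores the name and applies material, mass and half-factor scale to the sphere.
; Go sets a random negative X velocity, while Launch and Elevate add upward velocity at different strengths.
; Anchor makes the sphere very heavy and zeroes its velocity, and Victory destroys the actor.
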(event Custom|Go
  ;[1 1 1] Start Movement
  (Physics|SetPhysicsLinearVelocity (Variables|Default|GetSphere) (Math|Vector|MakeVector (Math|Random|RandomFloatinRange -3e+02 -6e+02) 0.0 0.0) false "None"))

(event Custom|Launch
  (params (velocity :type Float%20%28double-precision%29))
  ;[1 1 1] Launch
  (Physics|SetPhysicsLinearVelocity (Variables|Default|GetSphere) (Math|Vector|MakeVector 0.0 0.0 (* velocity 1.5e+03)) true "None"))

(event Custom|Victory
  (Actor|DestroyActor))

(event Custom|Initialize
  (params (Data :type ST%20MOB%20Structure))
  (bind _returnvalue (* (.scale Data) 0.5))
  (bind _sphere (Variables|Default|GetSphere))
  ;[1 1 1] Initialize
  (Utilities|FlowControl|Sequence
    (:then_0
      (Variables|Default|SetData%20Name (.name Data)))
    (:then_1
      (Rendering|Material|SetMaterial _sphere 0 (.color Data)))
    (:then_2
      (Class|PrimitiveComponent|SetMassOverrideinKg _sphere "None" (.mass Data) true))
    (:then_3
      (Transformation|SetWorldScale3D _sphere (Math|Vector|MakeVector _returnvalue _returnvalue _returnvalue)))))

(event Custom|Anchor
  (bind _sphere (Variables|Default|GetSphere))
  (Class|PrimitiveComponent|SetMassOverrideinKg _sphere "None" 1e+03 true)
  (Physics|SetPhysicsLinearVelocity _sphere "0, 0, 0" false "None"))

(event Custom|Elevate
  (params (Velocity :type Float%20%28double-precision%29))
  (bind _sphere (Variables|Default|GetSphere))
  (bind _returnvalue (Physics|GetPhysicsLinearVelocity _sphere "None"))
  (Physics|SetPhysicsLinearVelocity _sphere (Math|Vector|MakeVector (.x _returnvalue) (.y _returnvalue) (+ (.z _returnvalue) (* Velocity 5e+01))) false "None"))

(fn ConstructionScript)