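; Launcher actor that charges power and launches the BP_MOB_Base actors inside its overlap area.
; Overlap events maintain the MOB list, and on BeginPlay it enables player input and registers with a LevelController.
; While active, holding IA_Charge raises clamped Power and updates a text display; release or cancel launches every listed MOB with that power, then resets it.
; Start and Stop toggle activity, Reset clears the list, and a delay-based charging loop is left unused.
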(event Custom|OnActorBeginOverlap_Event
  (params (OverlappedActor :type Actor%20Object%20Reference) (OtherActor :type Actor%20Object%20Reference))
  ;[1 1 1] Add MOB to list
  (bind _asbp_mob_base (Utilities|Casting|CastToBP_MOB_Base OtherActor))
  (Utilities|Array|AddUnique (Variables|Default|GetMOBs) _asbp_mob_base))

(event Custom|OnActorEndOverlap_Event
  (params (OverlappedActor :type Actor%20Object%20Reference) (OtherActor :type Actor%20Object%20Reference))
  (bind _mobs (Variables|Default|GetMOBs))
  ;[1 1 1] Remove MOB from list when it leaves area
  (bind _asbp_mob_base (Utilities|Casting|CastToBP_MOB_Base OtherActor))
  (if (Utilities|Array|IsValidIndex _mobs (Utilities|Array|FindItem _mobs _asbp_mob_base))
    (Utilities|Array|RemoveItem _mobs _asbp_mob_base)))

(event Custom|Start
  (Variables|Default|SetActive true))

(event Custom|Stop
  (Variables|Default|SetActive false))

(event Custom|Reset
  (Utilities|Array|Clear (Variables|Default|GetMOBs)))

(event Input|EnhancedActionEvents|EnhancedInputActionIA_Charge
  (params (ActionValue :type Boolean) (ElapsedSeconds :type Float%20%28double-precision%29) (TriggeredSeconds :type Float%20%28double-precision%29) (InputAction :type Input%20Action%20Object%20Reference :default "/Game/FirstPerson/Input/Actions/IA_Charge.IA_Charge"))
  (bind _active (Variables|Default|GetActive))
  (:Ongoing
    ;[1 1 1] Charge Power
    (if _active
      (Variables|Default|SetPower (Math|Float|Clamp(Float) (+ (Variables|Default|GetPower) 0.01)))
      (CallFunction|UpdatePowerDisplay (Variables|Default|GetPower))))
  (:Canceled
    ;[1 1 1] Launch all MOBs in zone
    (if _active
      (if (> (Utilities|Array|Length (Variables|Default|GetMOBs)) 0) :!label _label
        (for _array_element (Variables|Default|GetMOBs)
          (Default|Launch _array_element (Variables|Default|GetPower))))
      (bind _output_get (Variables|Default|SetPower 0.0))
      (CallFunction|UpdatePowerDisplay _output_get)))
  (:Completed
    (if _active
      (goto _label))))

(event EventBeginPlay
  (bind _level_controller (Variables|Default|GetLevel%20Controller))
  (Utilities|FlowControl|Sequence
    (:then_0
      ;[1 1 1] Enable Input
      (Input|EnableInput (Game|GetPlayerController 0)))
    (:then_1
      ;[1 1 1] Initialize Power Display
      (CallFunction|UpdatePowerDisplay (Variables|Default|GetPower)))
    (:then_2
      (Utilities|FlowControl|Sequence
        (:then_0
          ;[1 1 1] Add MOB to list
          (EventDispatchers|BindEventtoOnActorBeginOverlap (delegate Custom|OnActorBeginOverlap_Event)))
        (:then_1
          ;[1 1 1] Remove MOB from list when it leaves area
          (EventDispatchers|BindEventtoOnActorEndOverlap (delegate Custom|OnActorEndOverlap_Event)))
        (:then_2
          (Utilities|IsValid _level_controller
            (:Is%20Valid
              (Default|RegisterLauncher _level_controller))))))))

(fn ConstructionScript)

(fn UpdatePowerDisplay
  (params (Value :type Float%20%28double-precision%29))
  (Rendering|Components|TextRender|SetText (Variables|Default|GetPower_Text) (Utilities|Text|FormatText "Power: {value}" Value)))