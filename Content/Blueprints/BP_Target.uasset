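; BP_Target is a target zone that detects mobs entering its BowlTarget component and registers itself with the LevelController on BeginPlay.
; Each overlapping actor is recorded once in Items; if it is a BP_MOB_Base, it is anchored, a hit sound plays and OnTargetHit is broadcast.
; Reset destroys every recorded actor, including non-mobs since recording precedes the cast, and empties the array.
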(event Custom|OnComponentBeginOverlap_Event
  (params (OverlappedComponent :type Primitive%20Component%20Object%20Reference) (OtherActor :type Actor%20Object%20Reference) (OtherComp :type Primitive%20Component%20Object%20Reference) (OtherBodyIndex :type Integer) (bFromSweep :type Boolean) (SweepResult :type Hit%20Result%20Structure%20%28by%20ref%29))
  (bind _items (Variables|Default|GetItems))
  ;[1 1 1] Trigger the event once per item
  (if (== (Utilities|Array|FindItem _items OtherActor) -1)
    (Utilities|Array|AddUnique _items OtherActor)
    (bind _asbp_mob_base (Utilities|Casting|CastToBP_MOB_Base OtherActor))
    (Default|Anchor _asbp_mob_base)
    (Audio|PlaySound2D "/Game/Sound/Music/Candy_Target_mixdown.Candy_Target_mixdown" 1.0 1.0 0.0 0 0 false)
    (Default|CallOnTargetHit _asbp_mob_base)))

(event Custom|Reset
  (bind _items (Variables|Default|GetItems))
  ;[1 1 1] Reset - Clear items and clear array
  (for _array_element _items
    (Utilities|IsValid _array_element
      (:Is%20Valid
        (Actor|DestroyActor _array_element))))
  (Utilities|Array|Clear _items))

(event EventBeginPlay
  (bind _level_controller (Variables|Default|GetLevel%20Controller))
  (Utilities|FlowControl|Sequence
    (:then_0
      (Collision|AssignOnComponentBeginOverlap (Variables|Default|GetBowlTarget) (delegate Custom|OnComponentBeginOverlap_Event)))
    (:then_1
      ;[1 1 1] Register
      (Utilities|IsValid _level_controller
        (:Is%20Valid
          (Default|RegisterTargetZone _level_controller self))))))

(fn ConstructionScript)