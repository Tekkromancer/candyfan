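; BP_Spawner is a mob spawner that registers with the LevelController and is controlled through Start, Stop and Reset events.
; While active, it loops on a random short delay, picks a random row from DT_MOBs and spawns a BP_MOB_Base at its Sphere's location.
; Each mob is initialized from that row, tracked in Items and told to Go.
; Stop ends the loop, and Reset destroys and clears all tracked mobs.
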(event Custom|Stop
  (Variables|Default|SetActive false))

(event Custom|Start
  (Variables|Default|SetActive true)
  (Utilities|FlowControl|Delay (Math|Random|RandomFloatinRange 1.0 3.0) :!label _label)
  ;[1 1 1] TODO: Spawn random instance
  (bind _returnvalue (Utilities|GetDataTableRow "/Game/Data/DT_MOBs.DT_MOBs" (.OutItem (Utilities|Array|Random (Variables|Default|GetMOB%20Names))))
    (:then
      (bind _returnvalue_2 (Game|SpawnActorfromClass "/Game/Blueprints/BP_MOB_Base.BP_MOB_Base_C" (Math|Conversions|ToTransform(Vector) (Transformation|GetWorldLocation (Variables|Default|GetSphere))) "Undefined" "MultiplyWithRoot" 0 0))
      (Utilities|FlowControl|Sequence
        (:then_0
          (Default|Initialize _returnvalue_2 _returnvalue))
        (:then_1
          (Utilities|Array|AddUnique (Variables|Default|GetItems) _returnvalue_2))
        (:then_2
          (Default|Go _returnvalue_2)
          (if (Variables|Default|GetActive)
            (goto _label)))))))

(event Custom|Reset
  (bind _items (Variables|Default|GetItems))
  (Utilities|FlowControl|Sequence
    (:then_0
      (for _array_element _items
        (Utilities|IsValid _array_element
          (:Is%20Valid
            (Actor|DestroyActor _array_element)))))
    (:then_1
      (Utilities|Array|Clear _items))))

(event EventBeginPlay
  (Utilities|FlowControl|Sequence
    (:then_0
      ;[1 1 1] Register
      (Default|RegisterSpawner (Variables|Default|GetLevel%20Controller) self))
    (:then_1
      (bind _outrownames (DataTable|GetDataTableRowNames "/Game/Data/DT_MOBs.DT_MOBs"))
      (Variables|Default|SetMOB%20Names _outrownames))))

(fn ConstructionScript)