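; BP_Launcher is a player-charged fan launcher that lifts MOB actors within its overlap area.
; Holding IA_Charge plays a timeline that raises Power and releasing reverses it, with Power also driving the fan's speed.
; Overlap events maintain the MOB list, and Tick calls Elevate with Power on each while active.
; It registers with the LevelController, whose start and game-complete events switch it on and off.
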(event Custom|OnActorBeginOverlap_Event
  (params (OverlappedActor :type Actor%20Object%20Reference) (OtherActor :type Actor%20Object%20Reference))
  ;[1 1 1] Add MOB to list
  (bind _asbp_mob_base (Utilities|Casting|CastToBP_MOB_Base OtherActor))
  (Utilities|Array|AddUnique (Variables|Default|GetMOBs) _asbp_mob_base))

(event Custom|OnActorEndOverlap_Event
  (params (OverlappedActor :type Actor%20Object%20Reference) (OtherActor :type Actor%20Object%20Reference))
  (bind _mobs (Variables|Default|GetMOBs))
  ;[1 1 1] Remove MOB from list when it leaves area
  (bind _asbp_mob_base (Utilities|Casting|CastToBP_MOB_Base OtherActor))
  (if (Utilities|Array|IsValidIndex _mobs (Utilities|Array|FindItem _mobs _asbp_mob_base))
    (Utilities|Array|RemoveItem _mobs _asbp_mob_base)))

(event Custom|Game%20Complete
  (CallFunction|Stop))

(event Custom|Start
  (Variables|Default|SetActive true))

(event Custom|Stop
  (Variables|Default|SetActive false)
  (Variables|Default|SetCharging false))

(event Custom|Reset
  (Utilities|Array|Clear (Variables|Default|GetMOBs))
  (Variables|Default|SetActive true))

(event Custom|OnStart
  (CallFunction|Start))

(event Input|EnhancedActionEvents|EnhancedInputActionIA_Charge
  (params (ActionValue :type Boolean) (ElapsedSeconds :type Float%20%28double-precision%29) (TriggeredSeconds :type Float%20%28double-precision%29) (InputAction :type Input%20Action%20Object%20Reference :default "/Game/FirstPerson/Input/Actions/IA_Charge.IA_Charge"))
  (bind _active (Variables|Default|GetActive))
  ;[1 1 1] Handle charge input
  (:Started
    (if _active
      (bind _power (Timeline|Power%20Timeline Play)
        (:Update
          (bind _output_get (Variables|Default|SetPower _power))
          (CallFunction|UpdatePowerDisplay _output_get)))))
  (:Completed
    (if _active
      (Timeline|Power%20Timeline Reverse))))

(event EventBeginPlay
  (bind _level_controller (Variables|Default|GetLevel%20Controller))
  (bind _level_controller_2 (Variables|Default|GetLevel%20Controller))
  (Utilities|FlowControl|Sequence
    (:then_0
      ;[1 1 1] Enable Input
      (Input|EnableInput (Game|GetPlayerController 0)))
    (:then_1
      ;[1 1 1] Initialize Power Display
      (CallFunction|UpdatePowerDisplay (Variables|Default|GetPower)))
    (:then_2
      (Utilities|FlowControl|Sequence
        (:then_0
          ;[1 1 1] Add MOB to list
          (EventDispatchers|BindEventtoOnActorBeginOverlap (delegate Custom|OnActorBeginOverlap_Event)))
        (:then_1
          ;[1 1 1] Remove MOB from list when it leaves area
          (EventDispatchers|BindEventtoOnActorEndOverlap (delegate Custom|OnActorEndOverlap_Event)))
        (:then_2
          (Utilities|IsValid _level_controller_2
            (:Is%20Valid
              (Default|RegisterLauncher _level_controller_2))))))
    (:then_4
      (Utilities|FlowControl|Sequence
        (:then_0
          (EventDispatchers|BindEventtoOnGameComplete _level_controller (delegate Custom|Game%20Complete)))
        (:then_1
          (EventDispatchers|BindEventtoOnStart _level_controller (delegate Custom|OnStart)))))))

(event EventTick
  (params (DeltaSeconds :type Float%20%28single-precision%29))
  ;[1 1 1] Launch all MOBs in zone and reset power to zero.
  (if (Variables|Default|GetActive)
    (if (> (Utilities|Array|Length (Variables|Default|GetMOBs)) 0)
      (for _array_element (Variables|Default|GetMOBs)
        (Default|Elevate _array_element (Variables|Default|GetPower))))))

(fn ConstructionScript)

(fn UpdatePowerDisplay
  (params (Value :type Float%20%28double-precision%29))
  (Variables|/Game/Blueprints/BP_Fan.BP_Fan_C|SetSpeed (Variables|Default|GetFan) Value))